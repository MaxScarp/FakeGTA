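; Actor component that tracks health and stamina for its owner, filling both to their maximums on BeginPlay.
; Increase functions clamp to the maximum and return the new value.
; Decrease functions return true when the value reaches zero or below.
; Only stamina is clamped at zero, so health can go negative.
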(event `self.ReceiveBeginPlay`
  (set `self.CurrentHealth` (`self.MaxHealth`))
  (set `self.CurrentStamina` (`self.MaxStamina`)))

(fn `DecreaseHealth`
  (params (Damage :type "Float (double-precision)"))
  (returns (IsDead :type Boolean))
  (bind _output_get (set `self.CurrentHealth` (- (`self.CurrentHealth`) Damage)))
  (if (<= _output_get 0.0)
    (return true)
    (else
      (return false))))

(fn `DecreaseStamina`
  (params (DecreasedStamina :type "Float (double-precision)"))
  (returns (IsStaminaNotLeft :type Boolean))
  (bind _output_get (set `self.CurrentStamina` (- (`self.CurrentStamina`) DecreasedStamina)))
  (if (<= _output_get 0.0)
    (set `self.CurrentStamina` 0.0)
    (return true)
    (else
      (return false))))

(fn `IncreaseHealth`
  (params (AddedHealth :type "Float (double-precision)"))
  (returns (NewHealth :type "Float (double-precision)"))
  (bind _maxhealth (`self.MaxHealth`))
  (bind _output_get (set `self.CurrentHealth` (+ (`self.CurrentHealth`) AddedHealth)))
  (if (> _output_get _maxhealth)
    (set `self.CurrentHealth` _maxhealth))
  (return (`self.CurrentHealth`)))

(fn `IncreaseStamina`
  (params (AddedStamina :type "Float (double-precision)"))
  (returns (NewStamina :type "Float (double-precision)"))
  (bind _maxstamina (`self.MaxStamina`))
  (bind _output_get (set `self.CurrentStamina` (+ (`self.CurrentStamina`) AddedStamina)))
  (if (> _output_get _maxstamina)
    (set `self.CurrentStamina` _maxstamina))
  (return (`self.CurrentStamina`)))