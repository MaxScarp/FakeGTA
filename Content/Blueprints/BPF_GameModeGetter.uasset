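; Blueprint helper functions that give access to the single-player game mode and its player reference.
; GetGameMode casts the current game mode to GM_SinglePlayer and returns it with a success flag.
; GetPlayerPawn builds on that to return the game mode's PlayerBlueprint, with success reflecting only the cast, not the reference's validity.
; Both print an error message on failure.
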(fn `GetGameMode`
  (returns (DoneSuccesfully :type Boolean) (GameModeRef :type "/Game/Blueprints/GM_SinglePlayer Object Reference"))
  (locals (Success :type Boolean :default true))
  (bind _asgm_single_player (cast `/Game/Blueprints/GM_SinglePlayer` (`GameplayStatics.GetGameMode` null))
    (:`then`
      (set `local.Success` true))
    (:`CastFailed`
      (`KismetSystemLibrary.PrintString` null "GAME MODE NOT FOUND!" true true (struct :`R` 1.0 :`G` 0.049243 :`A` 1.0) 10.0)
      (set `local.Success` false)))
  (return (`local.Success`) _asgm_single_player))

(fn `GetPlayerPawn`
  (returns (DoneSuccesfully :type Boolean) (PlayerBlueprintRef :type "/Game/Blueprints/BP_Player Object Reference"))
  (locals (DoneWithSuccess :type Boolean))
  (bind (_donesuccesfully _gamemoderef) (`self.GetGameMode` null))
  (if _donesuccesfully
    (set `local.DoneWithSuccess` true)
    (else
      (`KismetSystemLibrary.PrintString` null "PLAYER NOT AVAILABLE!" true true (struct :`R` 1.0 :`G` 0.049243 :`A` 1.0) 10.0)
      (set `local.DoneWithSuccess` false)))
  (return (`local.DoneWithSuccess`) (`/Game/Blueprints/GM_SinglePlayer.PlayerBlueprint` _gamemoderef)))